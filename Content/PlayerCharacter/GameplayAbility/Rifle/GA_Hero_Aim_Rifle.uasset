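; Gameplay ability for aiming the hero's rifle, currently reduced to debug prints when it activates and ends.
; An unconnected branch holds toggle logic that checks the combat component's RifleAimTag against AimTag, sets or clears that tag, updates the hero character's aiming state, then ends the ability.
; That toggle never runs, so activation neither changes aim state nor ends the ability itself.
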(event Ability|EventActivateAbility
  (Development|PrintString "Aim Ability Activated" true true "(R=0.000000,G=0.660000,B=1.000000,A=1.000000)" 6.0))

(event Ability|EventOnEndAbility
  (params (bWasCancelled :type Boolean))
  (Development|PrintString "Aim Ability Ended" true true "(R=0.000000,G=0.660000,B=1.000000,A=1.000000)" 6.0))